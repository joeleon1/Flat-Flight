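; Player Blueprint that flashes a damage overlay on screen and handles level restarts.
; Tick polls a DamageEffectSignal flag, creates a DamageTakenWidget, removes it after a short delay and clears the flag, with a guard bool preventing overlapping flashes.
; The Reset input action runs the RestartLevel console command, but only while the game is paused.
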(event EventTick
  (params (DeltaSeconds :type Float%20%28single-precision%29))
  (if (Variables|Default|GetdamageEffectSignal)
    (if (not (Variables|Default|GetisShowingDmgEffect))
      (Variables|Default|SetisShowingDmgEffect true)
      (bind _returnvalue (UserInterface|CreateWidget "/Game/Blueprints/DamageTakenWidget.DamageTakenWidget_C"))
      (UserInterface|Viewport|AddtoViewport _returnvalue 0)
      (Utilities|FlowControl|Delay 0)
      (Widget|RemovefromParent _returnvalue)
      (Variables|Default|SetdamageEffectSignal false)
      (Variables|Default|SetisShowingDmgEffect false))))

(event Input|ActionEvents|InputActionReset
  (params (Key :type Key%20Structure :default "AnyKey"))
  (:Pressed
    (if (Game|IsGamePaused)
      (Development|ExecuteConsoleCommand 0 "RestartLevel"))))

(fn ConstructionScript)